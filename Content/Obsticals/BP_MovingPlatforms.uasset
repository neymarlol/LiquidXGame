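; BP_MovingPlatforms is an obstacle platform that moves back and forth continuously from the start of play.
; A Timeline, with play rate and length set from Speed and Duration, drives a MovePlatform event that sets the static mesh's relative location to Direction times the track value.
; When the Timeline finishes, it waits briefly, then reverses or replays depending on the track value, creating a ping-pong loop.
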(event `self.ReceiveBeginPlay`
  (bind _timeline (`self.Timeline`))
  ;[1 1 1] Play speed
  (`TimelineComponent.SetPlayRate` _timeline (`self.Speed`))
  (`TimelineComponent.SetTimelineLength` _timeline (`self.Duration`))
  ;[1 1 1] Controlling move direction
  (bind (_direction _track) (`Timeline|Timeline` :!via `PlayFromStart` :!label _label)
    (:`Update`
      (`self.MovePlatform` _track))
    (:`Finished`
      (if (> _track 0.0)
        (`KismetSystemLibrary.Delay` 0.2)
        (goto _label :!via `Reverse`)
        (else
          (`KismetSystemLibrary.Delay` 0.2)
          (goto _label :!via `PlayFromStart`))))))

(event `MovePlatform`
  (params (Track :type "Float (double-precision)"))
  ;[1 1 1] Move platform logic
  (`SceneComponent.K2_SetRelativeLocation` (`self.StaticMesh`) (* (`self.Direction`) Track) false false))

(fn `UserConstructionScript`)